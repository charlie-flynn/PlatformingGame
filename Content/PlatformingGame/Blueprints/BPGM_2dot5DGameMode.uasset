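; Game mode for a 2.5D platformer that sets up the UI and supports respawning the player character.
; BeginPlay shows the UI, saves the player pawn's starting transform and binds its destruction to OnPlayerDeath, which is empty.
; RespawnPlayer spawns a new character at the saved location and rotation with a separate scale, possesses it and binds it to PathManager.
; Nothing here calls RespawnPlayer, and it does not rebind the destroyed event.
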(event `self.ReceiveBeginPlay`
  (bind _returnvalue (`GameplayStatics.GetPlayerPawn` 0))
  (`UserWidget.AddToViewport` (`self.UserInterface`) 0)
  (set `self.PlayerSpawnTransform` (`self.GetTransform` _returnvalue))
  (add `self.OnDestroyed` _returnvalue (delegate `On Player Death`)))

(event `On Player Death` :!signature `self.OnDestroyed`
  (params (DestroyedActor :type "Actor Object Reference")))

(fn `RespawnPlayer`
  (returns (Player :type "/Game/PlatformingGame/Blueprints/BP_2dot5DCharacter Object Reference"))
  (bind (_playerspawntransform_location _playerspawntransform_rotation) (`KismetMathLibrary.BreakTransform` (`self.PlayerSpawnTransform`)))
  (bind _returnvalue (`|SpawnActorFromClass` "/Game/PlatformingGame/Blueprints/BP_2dot5DCharacter.BP_2dot5DCharacter_C" (`KismetMathLibrary.MakeTransform` _playerspawntransform_location _playerspawntransform_rotation (`self.PlayerSpawnScale`)) "Undefined" "MultiplyWithRoot" null null))
  (`Controller.Possess` (`GameplayStatics.GetPlayerController` 0) _returnvalue)
  (`PathManager.BindActor` (`self.PathManager`) _returnvalue)
  (return _returnvalue))

(fn `UserConstructionScript`)