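; BP_2dot5DCamera is a side-scrolling camera actor for a 2.5D platformer that follows the player character along the world Y axis only.
; On BeginPlay it caches the player and its own starting location.
; Each Tick it matches the player's Y plus an Offset, holding X and Z at the base position plus Offset.
; It then subtracts Offset to store the base position again, so the offset does not accumulate.
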(event `self.ReceiveBeginPlay`
  (bind _returnvalue_location (`KismetMathLibrary.BreakTransform` (`self.GetTransform`)))
  (set `self.Player` (`GameplayStatics.GetPlayerCharacter` 0))
  (set `self.PreOffsetPosition` _returnvalue_location))

(event `self.ReceiveTick`
  (params (DeltaSeconds :type "Float (single-precision)"))
  (bind (_returnvalue_location _returnvalue_rotation _returnvalue_scale) (`KismetMathLibrary.BreakTransform` (`self.GetTransform`)))
  (bind _returnvalue (`self.GetTransform`))
  (bind (_offset_x _offset_y _offset_z) (`KismetMathLibrary.BreakVector` (`self.Offset`)))
  (bind (_preoffsetposition_x _preoffsetposition_y _preoffsetposition_z) (`KismetMathLibrary.BreakVector` (`self.PreOffsetPosition`)))
  (bind (_offset_x_2 _offset_y_2 _offset_z_2) (`KismetMathLibrary.BreakVector` (`self.Offset`)))
  (`self.K2_SetActorTransform` (`KismetMathLibrary.MakeTransform` (`KismetMathLibrary.MakeVector` (+ _preoffsetposition_x _offset_x_2) (+ (.y (.location (`self.GetTransform` (`self.Player`)))) _offset_y_2) (+ _offset_z_2 _preoffsetposition_z)) _returnvalue_rotation _returnvalue_scale))
  (set `self.PreOffsetPosition` (`KismetMathLibrary.MakeVector` (- (.x (.location _returnvalue)) _offset_x) (- (.y (.location _returnvalue)) _offset_y) (- (.z (.location _returnvalue)) _offset_z))))

(fn `UserConstructionScript`)